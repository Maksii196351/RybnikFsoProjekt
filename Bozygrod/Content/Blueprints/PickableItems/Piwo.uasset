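; Piwo (Polish for "beer") is a pickable-item actor for a bottle that shatters when it hits something fast enough.
; On StaticMesh component hit, it compares the mesh's velocity to a threshold, which is much lower for actors tagged "Ground" than for anything else.
; Above the threshold, it plays a breaking-glass sound at the mesh's location, prints a debug message and destroys itself.
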(event `self.ReceiveTick`
  (params (DeltaSeconds :type "Float (single-precision)")))

(event `self.StaticMesh.OnComponentHit`
  (params (HitComponent :type "PrimitiveComponent Object Reference") (OtherActor :type "Actor Object Reference") (OtherComp :type "PrimitiveComponent Object Reference") (NormalImpulse :type "Vector Structure") (Hit :type "HitResult Structure (by ref)"))
  (bind _returnvalue (`KismetMathLibrary.VSize` (`SceneComponent.GetComponentVelocity` (`self.StaticMesh`))))
  (if (`self.ActorHasTag` OtherActor "Ground")
    (if (> _returnvalue 100.0)
      (`GameplayStatics.PlaySoundAtLocation` "/Game/Sounds/BreakingGlass.BreakingGlass" (`SceneComponent.K2_GetComponentLocation` (`self.StaticMesh`)) (struct) 1.0 1.0 0.0 null null null null)
      (`KismetSystemLibrary.PrintString` "YouDestroyed a bottle")
      (`self.K2_DestroyActor`))
    (elif (> _returnvalue 400.0)
      (`GameplayStatics.PlaySoundAtLocation` "/Game/Sounds/BreakingGlass.BreakingGlass" (`SceneComponent.K2_GetComponentLocation` (`self.StaticMesh`)) (struct) 1.0 1.0 0.0 null null null null)
      (`KismetSystemLibrary.PrintString` "YouDestroyed a bottle")
      (`self.K2_DestroyActor`))))

(fn `UserConstructionScript`
  (`parent.UserConstructionScript`))