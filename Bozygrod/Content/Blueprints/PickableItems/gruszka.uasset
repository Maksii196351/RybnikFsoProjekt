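; Pickable pear item (gruszka) with an expiry value that can turn it into a rotten pear.
; Each Tick runs the parent logic, then subtracts a constant, shown as 0.0, from Datawaznosci, independent of DeltaSeconds.
; While that value is zero or below, it sets the static mesh to Zgnila_gruszka every frame.
; BeginPlay and overlap events are disabled stubs, and the construction script only calls its parent.
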(event `self.ReceiveTick`
  (params (DeltaSeconds :type "Float (single-precision)"))
  (`parent.ReceiveTick` DeltaSeconds)
  (bind _output_get (set `self.datawaznosci` (- (`self.datawaznosci`) 0.0)))
  (if (<= _output_get 0.0)
    (`StaticMeshComponent.SetStaticMesh` (`self.StaticMesh`) "/Game/Produkty/Stałe/gruszka/zgnila/zgnila_gruszka.zgnila_gruszka")))

(fn `UserConstructionScript`
  (`parent.UserConstructionScript`))