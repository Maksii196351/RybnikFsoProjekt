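; JAPKO is a pickable apple item that rots over time.
; Each Tick counts the Datawaznosci (expiry) timer down by delta seconds, and once it reaches zero or below, swaps the static mesh to the rotten apple, repeating that set every following tick.
; A TurnOffSim event disables physics simulation on the mesh.
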(event `self.ReceiveTick`
  (params (DeltaSeconds :type "Float (single-precision)"))
  (bind _output_get (set `self.datawaznosci` (- (`self.datawaznosci`) DeltaSeconds)))
  (if (<= _output_get 0.0)
    (`StaticMeshComponent.SetStaticMesh` (`self.StaticMesh`) "/Game/Produkty/Stałe/Jablko/zgnile/jabłko_zgnile.jabłko_zgnile")))

(event `/Game/Blueprints/BI_Products.TurnOffSim`
  (`PrimitiveComponent.SetSimulatePhysics` (`self.StaticMesh`) false))

(fn `UserConstructionScript`
  (`parent.UserConstructionScript`))