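; SER is a pickable cheese item that goes moldy once its expiry time runs out.
; Every tick it subtracts the frame's delta time from the DataWaznosci (expiry) countdown.
; At zero or below it swaps its static mesh to Serek_plesn, the moldy version, and repeats that call each tick because nothing stops the countdown.
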(event `self.ReceiveTick`
  (params (DeltaSeconds :type "Float (single-precision)"))
  (bind _output_get (set `self.DataWaznosci` (- (`self.DataWaznosci`) DeltaSeconds)))
  (if (<= _output_get 0.0)
    (`StaticMeshComponent.SetStaticMesh` (`self.StaticMesh`) "/Game/Produkty/Stałe/ser/serek_plesn.serek_plesn")))

(fn `UserConstructionScript`
  (`parent.UserConstructionScript`))