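; AI controller for client NPCs that starts their BT_ClientBase behavior tree shortly after possession.
; It then stores the player character in the Blackboard under the MoveToPlayerName key.
; It also casts the Blackboard's ObjectKey value to BP_ClientBase and, on success, assigns that same value to its WhatIsBuying.
; Tick prints a debug string showing the controller and the ObjectKey value, labeled as fruit.
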(event `self.ReceivePossess`
  (params (PossessedPawn :type "Pawn Object Reference"))
  (bind _blackboard (`self.Blackboard`))
  (bind _returnvalue (`BlackboardComponent.GetValueAsObject` _blackboard "ObjectKey"))
  (`KismetSystemLibrary.Delay` 0.2)
  (`self.RunBehaviorTree` "/Game/Blueprints/AI/BT_ClientBase.BT_ClientBase")
  (`BlackboardComponent.SetValueAsObject` _blackboard (`self.Move To Player Name`) (`GameplayStatics.GetPlayerCharacter` 0))
  (bind _asbp_client_base (cast `/Game/Blueprints/Client/BP_ClientBase` _returnvalue))
  (set `/Game/Blueprints/Client/BP_ClientBase.What Is Buying` _returnvalue _asbp_client_base))

(event `self.ReceiveTick`
  (params (DeltaSeconds :type "Float (single-precision)"))
  (bind _blackboard (`self.Blackboard`))
  (if (!= _blackboard null)
    (`KismetSystemLibrary.PrintString` (`KismetTextLibrary.Conv_TextToString` (`|FormatText` "actor{a} fruit{f}" self (`BlackboardComponent.GetValueAsObject` _blackboard "ObjectKey"))) true true (struct :`G` 0.66 :`B` 1.0 :`A` 1.0) 2.0 "debug")))

(fn `UserConstructionScript`)