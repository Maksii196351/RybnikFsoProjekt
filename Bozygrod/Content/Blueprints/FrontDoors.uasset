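; Front door actor that lets customers in and starts the night phase, triggered once when the player overlaps its box.
; NewCustomer opens the door, teleports the next pre-placed BP_ClientBase to the spawn point, closes it, and re-calls itself with delays until every client is in.
; In parallel, a timeline drives directional light intensity, then sends NIGHTMessage to actors tagged "Night".
; StartNight triggers that broadcast directly.
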(event `self.ReceiveBeginPlay`
  (`parent.ReceiveBeginPlay`))

(event `NewCustomer`
  (`self.OpenDoor`)
  (bind _outactors (`GameplayStatics.GetAllActorsOfClass` "/Game/Blueprints/Client/BP_ClientBase.BP_ClientBase_C"))
  (`self.K2_TeleportTo` :`self` (`|GetArrayItem` _outactors (`self.ClientsSpawned`)) :`DestLocation` (`SceneComponent.K2_GetComponentLocation` (`self.SpawnRef`)))
  (`/Engine/EditorBlueprintResources/StandardMacros.IncrementInt` (`self.ClientsSpawned`)
    (:`  `
      (`KismetSystemLibrary.Delay` 1.0)
      (`self.CloseDoor`)
      (if (< (`self.ClientsSpawned`) (`KismetArrayLibrary.Array_Length` _outactors))
        (`KismetSystemLibrary.Delay` 2.0)
        (`self.NewCustomer`)))))

(event `Start Night`
  (`|ExecutionSequence` :!label _label
    (:`then_0`
      (bind _outactors (`GameplayStatics.GetAllActorsWithTag` "Night"))
      (for _array_element _outactors
        (message `/Game/Blueprints/Interfaces/BI_DayEnd.NIGHT` _array_element)
        (`KismetSystemLibrary.PrintString` (`KismetSystemLibrary.GetDisplayName` _array_element))))
    (:`then_1`
      (`KismetSystemLibrary.PrintString` "Night Started"))))

(event `self.Box.OnComponentBeginOverlap`
  (params (OverlappedComponent :type "PrimitiveComponent Object Reference") (OtherActor :type "Actor Object Reference") (OtherComp :type "PrimitiveComponent Object Reference") (OtherBodyIndex :type Integer) (bFromSweep :type Boolean) (SweepResult :type "HitResult Structure (by ref)"))
  (`/Engine/EditorBlueprintResources/StandardMacros.DoOnce` false
    (:`Completed`
      (if (== OtherActor (`GameplayStatics.GetPlayerPawn` 0))
        (`|ExecutionSequence`
          (:`then_0`
            (`KismetSystemLibrary.Delay` 2.0)
            (`self.NewCustomer`))
          (:`then_1`
            (bind (_direction _newtrack_0) (`Timeline|Timeline_0`)
              (:`Update`
                (`LightComponent.SetIntensity` (`self.DirectionalLight`) _newtrack_0))
              (:`Finished`
                (goto _label)))))))))

(fn `UserConstructionScript`
  (`parent.UserConstructionScript`))