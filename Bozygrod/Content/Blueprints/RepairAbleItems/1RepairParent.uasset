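; Base repairable-item actor that trades player resources for repairs up to a maximum count, with an empty Repaired event as a hook.
; A box overlap toggles a widget showing the current cost to the player.
; Repair compares resources, sends negated costs to the player, plays a sound, then after a delay compounds the cost by a growing, clamped multiplier.
; A DoOnce blocks re-entry, and the widget is destroyed at the limit.
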(event `self.ReceiveBeginPlay`
  (`StaticMeshComponent.SetStaticMesh` (`self.StaticMesh`) (`self.New Mesh`))
  (bind _returnvalue (`|CreateWidget` "/Game/Blueprints/RepairAbleItems/ResourcesNeeded.ResourcesNeeded_C"))
  (set `self.WidgetRef` _returnvalue)
  (`WidgetComponent.SetWidget` (`self.Widget`) _returnvalue)
  (set `self.RepairResources` (`self.BaseResourcesNeeded`))
  (`KismetSystemLibrary.Delay` 0.2)
  (message `/Game/Blueprints/BI_WidgetInfo.WidgetInfo` (`self.WidgetRef`) (`self.RepairResources`)))

(event `Repaired`
  (params (Repairs :type Integer)))

(event `self.ReceiveTick`
  (params (DeltaSeconds :type "Float (single-precision)")))

(event `/Game/Blueprints/BI_Buying.Repair`
  (params (Player :type "/Game/Blueprints/BP_Player Object Reference") (PlayerResources :type "Map of /Game/Blueprints/ENUM_ResourceType Enum to Integer" :default _))
  (bind _returnvalue_location (`KismetMathLibrary.BreakTransform` (`self.GetTransform`)))
  (bind _baseresourcesneeded (`self.BaseResourcesNeeded`))
  (bind _repairresources (`self.RepairResources`))
  (bind _repairresources_2 (`self.RepairResources`))
  (bind _returnvalue (not (>= (`self.Repairs`) (`self.MaxRepairTimes`))))
  (`KismetSystemLibrary.PrintString` (`KismetStringLibrary.Conv_BoolToString` _returnvalue))
  (if _returnvalue
    (`/Engine/EditorBlueprintResources/StandardMacros.DoOnce` false :!label _label
      (:`Completed`
        (set `self.Player Resources` PlayerResources)
        (bind _keys (`BlueprintMapLibrary.Map_Keys` (`self.Player Resources`)))
        (for _array_element _keys
          _)
        (if (>= (`BlueprintMapLibrary.Map_Find` (`self.Player Resources`) _array_element) (`BlueprintMapLibrary.Map_Find` _repairresources _array_element))
          (bind _keys_2 (`BlueprintMapLibrary.Map_Keys` _repairresources))
          (for _array_element_2 _keys_2
            (`BlueprintMapLibrary.Map_Add` _repairresources_2 _array_element_2 (* (`BlueprintMapLibrary.Map_Find` _repairresources_2 _array_element_2) -1)))
          (message `/Game/Blueprints/BI_PlayerItems.IncrementResource` Player (`self.RepairResources`) 0)
          (`GameplayStatics.PlaySoundAtLocation` (`self.Sound`) _returnvalue_location (struct) 1.0 1.0 0.0 null null null null)
          (`KismetSystemLibrary.Delay` (`self.Delay`))
          (bind _keys_3 (`BlueprintMapLibrary.Map_Keys` _baseresourcesneeded))
          (for _array_element_3 _keys_3
            (`BlueprintMapLibrary.Map_Add` _baseresourcesneeded _array_element_3 (* (`BlueprintMapLibrary.Map_Find` _baseresourcesneeded _array_element_3) (`self.ValueMultiplayer`))))
          (set `self.ValueMultiplayer` (`KismetMathLibrary.FClamp` (* (`self.ValueMultiplayer`) (`self.Increasing multiplayer`)) 0.0 3.0))
          (bind _output_get (set `self.RepairResources` _baseresourcesneeded))
          (message `/Game/Blueprints/BI_WidgetInfo.WidgetInfo` (`self.WidgetRef`) _output_get)
          (bind _result (`/Engine/EditorBlueprintResources/StandardMacros.IncrementInt` (`self.Repairs`))
            (:`  `
              (`self.Repaired` _result)
              (if (>= (`self.Repairs`) (`self.MaxRepairTimes`))
                (`ActorComponent.K2_DestroyComponent` (`self.Widget`))
                (else
                  (goto _label :!via `Reset`))))))))))

(event `self.Box.OnComponentBeginOverlap`
  (params (OverlappedComponent :type "PrimitiveComponent Object Reference") (OtherActor :type "Actor Object Reference") (OtherComp :type "PrimitiveComponent Object Reference") (OtherBodyIndex :type Integer) (bFromSweep :type Boolean) (SweepResult :type "HitResult Structure (by ref)"))
  (if (== OtherActor (`GameplayStatics.GetPlayerPawn` 0))
    (`SceneComponent.SetHiddenInGame` (`self.Widget`) false false)))

(event `self.Box.OnComponentEndOverlap`
  (params (OverlappedComponent :type "PrimitiveComponent Object Reference") (OtherActor :type "Actor Object Reference") (OtherComp :type "PrimitiveComponent Object Reference") (OtherBodyIndex :type Integer))
  (if (== OtherActor (`GameplayStatics.GetPlayerPawn` 0))
    (`SceneComponent.SetHiddenInGame` (`self.Widget`) true false)))

(fn `UserConstructionScript`)