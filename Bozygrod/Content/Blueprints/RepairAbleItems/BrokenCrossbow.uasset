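; Broken crossbow repairable item that is replaced by another actor once it is repaired.
; Its AfterRepair event spawns the class in WhatToSpawn0 at the item's location with a fixed rotation and half scale, ignoring collisions, then destroys itself.
; The rest of the repair logic is not in this graph, and BeginPlay, overlap and Tick are disabled stubs.
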(event `After Repair_1`
  (params (BaseResourcesNeeded :type "Map of /Game/Blueprints/ENUM_ResourceType Enum to Integer" :default _) (WidgetRef :type "/Game/Blueprints/RepairAbleItems/ResourcesNeeded Object Reference"))
  (bind _returnvalue_location (`KismetMathLibrary.BreakTransform` (`self.GetTransform`)))
  (`|SpawnActorFromClass` (`self.What to spawn_0`) (`KismetMathLibrary.MakeTransform` _returnvalue_location (struct :`Yaw` 180.0) (0.5 0.5 0.5)) "AlwaysSpawn" "MultiplyWithRoot" null null)
  (`self.K2_DestroyActor`))

(fn `UserConstructionScript`
  (`parent.UserConstructionScript`))