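; Repairable item Blueprint, pulka, that switches to its Pulka3 mesh and drops its interaction components once repairs are done.
; Shortly after BeginPlay, it checks whether Repairs has reached MaxRepairTimes and, if so, applies that finished state.
; The AfterRepairs event jumps to the same logic, setting the static mesh and destroying the Widget and Box components.
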(event `self.ReceiveBeginPlay`
  (`parent.ReceiveBeginPlay`)
  (`KismetSystemLibrary.Delay` 0.2)
  (if (>= (`self.Repairs`) (`self.MaxRepairTimes`))
    (`StaticMeshComponent.SetStaticMesh` (`self.StaticMesh`) "/Game/sciana_i_Podloga/Szafki/pulka3.pulka3" :!label _label)
    (`ActorComponent.K2_DestroyComponent` (`self.Widget`))
    (`ActorComponent.K2_DestroyComponent` (`self.Box`))))

(event `self.AfterRepairs`
  (goto _label))

(fn `UserConstructionScript`
  (`parent.UserConstructionScript`))