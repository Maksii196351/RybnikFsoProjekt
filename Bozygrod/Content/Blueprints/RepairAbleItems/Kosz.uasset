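; Repairable basket (Kosz) that stores fruit once it has been fixed.
; It binds to a repair event on BeginPlay, which swaps the basket to a wood material, makes its collision physics-only and marks it repaired.
; When repaired, actors tagged Fruit entering the capsule are released from the player's physics handle, sent a stop-simulation message and snapped to the basket's next socket, tracked by an attached-fruit counter.
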(event `self.ReceiveTick`
  (params (DeltaSeconds :type "Float (single-precision)")))

(event `self.Capsule.OnComponentBeginOverlap`
  (params (OverlappedComponent :type "PrimitiveComponent Object Reference") (OtherActor :type "Actor Object Reference") (OtherComp :type "PrimitiveComponent Object Reference") (OtherBodyIndex :type Integer) (bFromSweep :type Boolean) (SweepResult :type "HitResult Structure (by ref)"))
  (if (`self.IsRepaired`)
    (if (`self.ActorHasTag` OtherActor "Fruit")
      (bind _asbp_player (cast `/Game/Blueprints/BP_Player` (`GameplayStatics.GetPlayerPawn` 0)))
      (`PhysicsHandleComponent.ReleaseComponent` (`/Game/Blueprints/BP_Player.PhysicsHandle` _asbp_player))
      (message `/Game/Blueprints/BI_Products.TurnOffSim` OtherActor)
      (`self.K2_AttachToComponent` OtherActor (`self.Kosz_0`) (`|GetArrayItem` (`SceneComponent.GetAllSocketNames` (`self.Kosz_0`)) (`self.Attached fruit`)) "SnapToTarget" "SnapToTarget" "KeepRelative" false)
      (`/Engine/EditorBlueprintResources/StandardMacros.IncrementInt` (`self.Attached fruit`)))))

(event `self.ReceiveBeginPlay`
  (add `self.Repair` (delegate `RepairedBasketInsideBasketBP`)))

(event `RepairedBasketInsideBasketBP`
  (`PrimitiveComponent.SetMaterial` (`self.Kosz_0`) 0 "/Game/_GENERATED/MaksDzio/drewno.drewno")
  (`PrimitiveComponent.SetCollisionEnabled` (`self.Kosz_0`) "PhysicsOnly")
  (set `self.IsRepaired` true))

(fn `UserConstructionScript`)