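; RepairOnce is a repairable item that is replaced by another actor after it is repaired.
; On BeginPlay it runs the parent logic and sets its static mesh to NewMesh0.
; The AfterRepairs event spawns the WhatToSpawn0 class at the item's location at half scale, ignoring collisions, then destroys the item.
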(event `self.ReceiveBeginPlay`
  (`parent.ReceiveBeginPlay`)
  (`StaticMeshComponent.SetStaticMesh` (`self.StaticMesh`) (`self.New Mesh_0`)))

(event `self.AfterRepairs`
  (bind _returnvalue_location (`KismetMathLibrary.BreakTransform` (`self.GetTransform`)))
  (`|SpawnActorFromClass` (`self.What to spawn_0`) (`KismetMathLibrary.MakeTransform` _returnvalue_location (`self.Spawn Transform Rotation`) (0.5 0.5 0.5)) "AlwaysSpawn" "MultiplyWithRoot" null null)
  (`self.K2_DestroyActor`))

(fn `UserConstructionScript`
  (`parent.UserConstructionScript`))