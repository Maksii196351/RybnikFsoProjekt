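; BasketForFruits is a repairable fruit basket item built from four basket components.
; The Repaired event uses the repair count to select one basket component, switches its material to wood (Drewno) and sets its collision to query only.
; AfterRepairs destroys the Box and Widget components.
; BeginPlay, overlap and Tick are disabled stubs, and the construction script only calls its parent.
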(event `self.Repaired`
  (params (Repairs :type Integer))
  (bind _output (`|GetArrayItem` (`|MakeArray` null (`self.FirstBasket`) (`self.Basket2`) (`self.Basket3`) (`self.LastBasket`)) Repairs))
  (`PrimitiveComponent.SetMaterial` _output 0 "/Game/_GENERATED/MaksDzio/drewno.drewno")
  (`PrimitiveComponent.SetCollisionEnabled` _output "QueryOnly"))

(event `self.AfterRepairs`
  (`ActorComponent.K2_DestroyComponent` (`self.Box`))
  (`ActorComponent.K2_DestroyComponent` (`self.Widget`)))

(fn `UserConstructionScript`
  (`parent.UserConstructionScript`))