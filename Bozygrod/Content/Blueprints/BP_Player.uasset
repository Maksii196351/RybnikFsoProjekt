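; First-person-style player Blueprint that handles movement, look, item interaction, carried products, a weapon and a money/resource inventory.
; A camera line trace each Tick sets the item in front, which E routes to buy, repair or pickup interface messages.
; Product and Wepon events handle physics-handle carrying with scroll-adjusted distance and weapon attachment, with key 1 swapping between hand and back.
; Resource purchases deduct money and, like weapon changes, update the UI widget.
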(event `InputAxis|Forward`
  (params (AxisValue :type "Float (single-precision)"))
  ;[1 1 1] Walking + cam
  (`self.AddMovementInput` (`self.GetActorForwardVector`) AxisValue))

(event `self.ReceiveBeginPlay`
  (`|ExecutionSequence`
    (:`then_1`
      (bind _returnvalue (`|CreateWidget` "/Game/Blueprints/UI.UI_C"))
      (bind _output_get (set `self.UIRef` _returnvalue))
      (`UserWidget.AddToViewport` _output_get 0))
    (:`then_2`
      (set `self.PlayerProductRange` (`self.BaseProduct Range`)))
    (:`then_3`
      (bind _asplayer_controller (cast `PlayerController` (`GameplayStatics.GetPlayerController` 0)))
      (bind _returnvalue_2 (pcsubsystem `EnhancedInputLocalPlayerSubsystem` _asplayer_controller))
      (`/Engine/EditorBlueprintResources/StandardMacros.IsValid` _returnvalue_2
        (:`Is Valid`
          (`EnhancedInputSubsystemInterface.AddMappingContext` _returnvalue_2 "/Game/Blueprints/Controlls/PlayerConfig.PlayerConfig" 0 (struct)))))))

(event `InputAxis|Right`
  (params (AxisValue :type "Float (single-precision)"))
  ;[1 1 1] Walking + cam
  (`self.AddMovementInput` (`self.GetActorRightVector`) AxisValue))

(event `InputAxis|Turn`
  (params (AxisValue :type "Float (single-precision)"))
  ;[1 1 1] Walking + cam
  (`self.AddControllerYawInput` AxisValue))

(event `InputAxis|lookup`
  (params (AxisValue :type "Float (single-precision)"))
  ;[1 1 1] Walking + cam
  (`self.AddControllerPitchInput` AxisValue))

(event `Key|E`
  (params (Key :type "Key Structure"))
  (bind _iteminfront (`self.ItemInFront`))
  ;[1 1 1] Pickup
  (:`Pressed`
    (if (`self.WeponInHand`)
      _
      (elif (`KismetSystemLibrary.DoesImplementInterface` (`self.ItemInFront`) "/Game/Blueprints/Buying.Buying_C")
        (`|ExecutionSequence`
          (:`then_0`
            (bind _asbuying_parent (cast `/Game/Kupiec/BuyingParent` (`self.ItemInFront`)))
            (message `/Game/Blueprints/Buying.CanBuy` (`self.ItemInFront`) (`self.Money`) (`/Game/Kupiec/BuyingParent.eResourceType` _asbuying_parent) self))
          (:`then_1`
            (bind _asrepair_parent (cast `/Game/kusza/BrokenCrossbow/RepairParent` _iteminfront))
            (message `/Game/Blueprints/Buying.Repair` _iteminfront (`/Game/kusza/BrokenCrossbow/RepairParent.RepairResources` _asrepair_parent) self)))
        (else
          (message `/Game/Blueprints/Pickable.PickUp` (`self.ItemInFront`) self)))))
  (:`Released`
    (if (`self.ProductInHand`)
      (`PhysicsHandleComponent.ReleaseComponent` (`self.PhysicsHandle`))
      (set `self.ProductInHand` false)
      (set `self.PlayerProductRange` (`self.BaseProduct Range`)))))

(event `self.ReceiveTick`
  (params (DeltaSeconds :type "Float (single-precision)"))
  (bind _camera (`self.Camera`))
  (bind _camera_2 (`self.Camera`))
  (bind _returnvalue (`SceneComponent.K2_GetComponentLocation` _camera))
  ;[1 1 1] Pickup
  (`|ExecutionSequence`
    (:`then_0`
      (`KismetSystemLibrary.PrintText` (`|FormatText` "PrintFrom {Player}     WeponInHand {wepon}" self (`self.WeponInHand`)) true true (struct :`G` 0.66 :`B` 1.0 :`A` 1.0) 2.0 "player")
      (bind _outhit (`KismetSystemLibrary.LineTraceSingle` :`Start` _returnvalue :`End` (+ _returnvalue (* (`SceneComponent.GetForwardVector` _camera) 300.0)) :`TraceChannel` "TraceTypeQuery1" :`DrawDebugType` "ForDuration"))
      (set `self.ItemInFront` (`.HitActor` (`GameplayStatics.BreakHitResult` _outhit))))
    (:`then_1`
      (if (`self.ProductInHand`)
        (`PhysicsHandleComponent.SetTargetLocation` (`self.PhysicsHandle`) (+ (`SceneComponent.K2_GetComponentLocation` _camera_2) (* (`SceneComponent.GetForwardVector` _camera_2) (`self.PlayerProductRange`))))))
    (:`then_2`
      (`KismetSystemLibrary.PrintString` (`KismetTextLibrary.Conv_TextToString` (`|FormatText` "Base{R}Player{RR}" (`self.BaseProduct Range`) (`self.PlayerProductRange`))) true true (struct :`G` 0.66 :`B` 1.0 :`A` 1.0) 2.0 "range"))
    (:`then_3`
      (`KismetSystemLibrary.PrintString` (`KismetStringLibrary.Conv_IntToString` (`self.Money`)) true true (struct :`G` 0.66 :`B` 1.0 :`A` 1.0) 2.0 "money"))))

(event `/Game/Blueprints/PlayerItems.Product`
  ;[1 1 1] Pickup
  (if (not (`self.WeponInHand`))
    (set `self.ProductInHand` true)
    (`PhysicsHandleComponent.GrabComponentAtLocationWithRotation` (`self.PhysicsHandle`) (`.HitComponent` (`GameplayStatics.BreakHitResult` (stale `self.ReceiveTick` _outhit))) "None" (`SceneComponent.K2_GetComponentLocation` (`.HitComponent` (`GameplayStatics.BreakHitResult` (stale `self.ReceiveTick` _outhit)))) (`SceneComponent.K2_GetComponentRotation` (`.HitComponent` (`GameplayStatics.BreakHitResult` (stale `self.ReceiveTick` _outhit)))))))

(event `Key|One`
  (params (Key :type "Key Structure"))
  (:`Pressed`
    (if (`self.hasWepon`)
      (if (`self.ProductInHand`)
        _
        (elif (`self.WeponInHand`)
          (`self.K2_AttachToComponent` (`self.actual wepon`) (`self.BackREF`) "None" "SnapToTarget" "SnapToTarget" "SnapToTarget" true)
          (message `/Game/Blueprints/HUDInfo.PlayerHaveWeponInHand` (`self.UIRef`) false)
          (set `self.WeponInHand` false)
          (else
            (`self.K2_AttachToComponent` (`self.actual wepon`) (`self.HandRef`) "None" "SnapToTarget" "SnapToTarget" "SnapToTarget" true)
            (message `/Game/Blueprints/HUDInfo.PlayerHaveWeponInHand` (`self.UIRef`) true)
            (set `self.WeponInHand` true)))))))

(event `EnhancedInput|/Game/Blueprints/Controlls/Scroll`
  (params (ActionValue :type "Float (double-precision)") (ElapsedSeconds :type "Float (double-precision)") (TriggeredSeconds :type "Float (double-precision)") (InputAction :type "InputAction Object Reference" :default "/Game/Blueprints/Controlls/Scroll.Scroll"))
  (:`Triggered`
    (set `self.PlayerProductRange` (`KismetMathLibrary.FClamp` (+ (`self.PlayerProductRange`) (* ActionValue 10.0)) 50.0 250.0))))

(event `/Game/Blueprints/PlayerItems.Wepon`
  (params (WeponRef :type "Actor Object Reference") (IsRange :type Boolean) (Demage :type Integer) (reload :type Integer))
  (set `self.hasWepon` true)
  (set `self.WeponInHand` true)
  (set `self.actual wepon` WeponRef)
  (`self.K2_AttachToComponent` WeponRef (`self.HandRef`) "None" "SnapToTarget" "SnapToTarget" "SnapToTarget" true)
  (message `/Game/Blueprints/HUDInfo.PlayerHaveWepon` (`self.UIRef`) (`self.hasWepon`) WeponRef))

(event `/Game/Blueprints/PlayerItems.IncrementResource`
  (params (enResourcetype :type "/Game/Blueprints/ENUM_ResourceType Enum" :default "NewEnumerator0") (ammount :type Integer) (iPrice :type Integer))
  (switch `/Game/Blueprints/ENUM_ResourceType` enResourcetype
    (:`NewEnumerator0`
      (set `self.Wood_0` (+ (`self.Wood_0`) ammount)))
    (:`NewEnumerator1`
      (set `self.Steel_0` (+ (`self.Steel_0`) ammount)))
    (:`NewEnumerator2`
      (set `self.Rope_0` (+ (`self.Rope_0`) ammount))))
  (bind _output_get (set `self.Money` (- (`self.Money`) iPrice)))
  (message `/Game/Blueprints/HUDInfo.PlayerFeedback` (`self.UIRef`) self enResourcetype _output_get))

(fn `PickupAndBuy`
  (params (TestObject :type "Object Object Reference") (self2 :type "Object Object Reference") (self3 :type "Object Object Reference"))
  (if (`KismetSystemLibrary.DoesImplementInterface` TestObject "/Game/Blueprints/Buying.Buying_C")
    (bind _asbuying_parent (cast `/Game/Kupiec/BuyingParent` TestObject))
    (message `/Game/Blueprints/Buying.CanBuy` TestObject (`self.Money`) (`/Game/Kupiec/BuyingParent.eResourceType` _asbuying_parent) self)
    (else
      (message `/Game/Blueprints/Pickable.PickUp` self3 self))))

(fn `UserConstructionScript`)