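; DoorTemplateParent is a door Blueprint, named as a parent template, that toggles open and closed when its PickUp event fires.
; PickUp checks the IsOpen flag and calls OpenDoor or CloseDoor, which update the flag and play or reverse one Timeline.
; The Timeline's track drives the yaw of the Pivot's relative rotation on each update, followed by a Delay that leads to nothing.
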(event `/Game/Blueprints/Pickable.PickUp`
  (params (inneractor :type "Actor Object Reference"))
  (if (`self.is open`)
    (`self.CloseDoor`)
    (else
      (`self.OpenDoor`))))

(event `OpenDoor`
  (set `self.is open` true)
  (bind (_direction _newtrack_0) (`Timeline|Timeline` :!label _label)
    (:`Update`
      (`SceneComponent.K2_SetRelativeRotation` (`self.pivot`) (`KismetMathLibrary.MakeRotator` 0.0 0.0 _newtrack_0) false false)
      (`KismetSystemLibrary.Delay` 2.0))))

(event `CloseDoor`
  (set `self.is open` false)
  (goto _label :!via `Reverse`))

(fn `UserConstructionScript`)