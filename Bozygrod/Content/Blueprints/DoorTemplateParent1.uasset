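; Parent template Blueprint for a door that toggles open and closed when its PickUp event fires.
; PickUp checks the IsOpen flag and calls either OpenDoor or CloseDoor, which update the flag and play or reverse a shared Timeline.
; The Timeline drives the Pivot component's roll and Y position at a fixed height, so the door rotates and shifts together.
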(event `self.ReceiveBeginPlay`)

(event `/Game/Blueprints/Interfaces/BI_Pickable.PickUp`
  (params (inneractor :type "Actor Object Reference"))
  (if (`self.is open`)
    (`self.close door`)
    (else
      (`self.OpenDoor`))))

(event `OpenDoor`
  (bind _pivot (`self.pivot`))
  (set `self.is open` true)
  (bind (_direction _rotation _position) (`Timeline|Timeline` :!label _label)
    (:`Update`
      (`SceneComponent.K2_SetRelativeRotation` _pivot (`KismetMathLibrary.MakeRotator` _rotation) false false)
      (`SceneComponent.K2_SetRelativeLocation` _pivot (`KismetMathLibrary.MakeVector` 0.0 _position 306.0) false false))))

(event `close door`
  (set `self.is open` false)
  (goto _label :!via `Reverse`))

(fn `UserConstructionScript`)