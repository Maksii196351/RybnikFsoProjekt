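; Base client character that takes fruit, pays the player, and can be shot dead.
; A live client hit by a "Jabko"-tagged fruit destroys it and flags its want as met, while any fruit entering TakeRange is destroyed for a small random payout.
; Being shot ragdolls the mesh, after which PickUp sends a product message to the interactor.
; An ask montage calls an animation-end handler when completed or interrupted.
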(event `self.ReceiveBeginPlay`)

(event `self.CapsuleComponent.OnComponentHit`
  (params (HitComponent :type "PrimitiveComponent Object Reference") (OtherActor :type "Actor Object Reference") (OtherComp :type "PrimitiveComponent Object Reference") (NormalImpulse :type "Vector Structure") (Hit :type "HitResult Structure (by ref)"))
  (if (`self.bIsAlive`)
    (if (and (`self.ActorHasTag` OtherActor "Fruit") (`self.ActorHasTag` OtherActor "Jabko"))
      (`self.K2_DestroyActor` OtherActor)
      (set `self.Have what he want` true))))

(event `/Game/Blueprints/BI_NPC.GotShoot`
  (set `self.bIsAlive` false)
  (`PrimitiveComponent.SetSimulatePhysics` (`self.Mesh`) true)
  (`PrimitiveComponent.SetCollisionResponseToChannel` (`self.Mesh`) "ECC_Pawn" "ECR_Overlap"))

(event `/Game/Blueprints/BI_Pickable.PickUp`
  (params (inneractor :type "Actor Object Reference"))
  (if (not (`self.bIsAlive`))
    (message `/Game/Blueprints/BI_Player.Product` inneractor)))

(event `AskAnimation`
  (`|PlayMontage` (`self.Mesh`) "/Game/models/AskAnimation.AskAnimation"
    (:`OnCompleted`
      _)
    (:`OnInterrupted`
      _))
  (`self.OnAnimationEnd`))

(event `self.TakeRange.OnComponentBeginOverlap`
  (params (OverlappedComponent :type "PrimitiveComponent Object Reference") (OtherActor :type "Actor Object Reference") (OtherComp :type "PrimitiveComponent Object Reference") (OtherBodyIndex :type Integer) (bFromSweep :type Boolean) (SweepResult :type "HitResult Structure (by ref)"))
  (if (`self.ActorHasTag` OtherActor "Fruit")
    (`self.K2_DestroyActor` OtherActor)
    (message `/Game/Blueprints/BI_Player.IncrementMoney` (`GameplayStatics.GetPlayerPawn` 0) (`KismetMathLibrary.RandomIntegerInRange` 1 5))))

(fn `UserConstructionScript`)