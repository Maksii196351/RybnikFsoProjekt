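; SZOp is an actor whose Cube appears at a random spot when its NIGHT event fires, then keeps facing the player.
; NIGHT teleports the Cube to one of four scene component locations, unhides it and sets IsSpawned.
; While IsSpawned is true, Tick turns the Cube toward the player character's capsule with a look-at rotation.
; Nothing in this Blueprint calls NIGHT or hides the Cube again.
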(event `self.ReceiveTick`
  (params (DeltaSeconds :type "Float (single-precision)"))
  (bind _cube (`self.Cube`))
  (if (`self.bIsSpawned`)
    (`SceneComponent.K2_SetWorldRotation` _cube (`KismetMathLibrary.FindLookAtRotation` (`SceneComponent.K2_GetComponentLocation` _cube) (`SceneComponent.K2_GetComponentLocation` (`Character.CapsuleComponent` (`GameplayStatics.GetPlayerCharacter` 0)))) false false)))

(event `/Game/Blueprints/Interfaces/BI_DayEnd.NIGHT`
  (bind _cube (`self.Cube`))
  (`SceneComponent.K2_SetWorldLocation` _cube (`SceneComponent.K2_GetComponentLocation` (`|GetArrayItem` (`|MakeArray` (`self.Scene2`) (`self.Scene1`) (`self.Scene`) (`self.Scene3`)) (`KismetMathLibrary.RandomIntegerInRange` 0 3))) false false)
  (`SceneComponent.SetHiddenInGame` _cube false false)
  (set `self.bIsSpawned` true))

(fn `UserConstructionScript`)